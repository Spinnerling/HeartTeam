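; Pusher actor that moves its static mesh when the player character overlaps it, apparently as a pushing trap or obstacle.
; It caches the mesh's world location at BeginPlay, then on overlap waits 0.2 seconds and restarts a timeline.
; Each timeline update sets the mesh location, without sweep, by interpolating between the Hitbox location and the cached start position.
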(event Collision|EventActorBeginOverlap
  (params (OtherActor :type Actor%20Object%20Reference))
  (if (== (Game|GetPlayerCharacter 0) OtherActor)
    (Utilities|FlowControl|Delay 0.2)
    (bind _wawdasd (Timeline|Timeline_0 PlayFromStart)
      (:Update
        (Transformation|SetWorldLocation (Variables|Default|GetStaticMesh) (Math|Vector|Lerp(Vector) (Transformation|GetWorldLocation (Variables|Default|Gethitbox)) (Variables|Default|Getinit_position) _wawdasd) false false)))))

(event EventBeginPlay
  (Variables|Default|Setinit_position (Transformation|GetWorldLocation (Variables|Default|GetStaticMesh))))

(fn ConstructionScript)