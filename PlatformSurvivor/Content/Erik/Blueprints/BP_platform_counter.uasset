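; BP_platform_counter is a counter meant to track destroyed platforms toward a win condition.
; On BeginPlay it stores the number of actors tagged "Platform" as the total.
; Its own Destroyed event, not one bound to the platforms, increments and prints the destroyed count, then compares it to the total.
; The win branch is still empty.
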(event EventBeginPlay
  ;[1 1 1] Find all platforms when the game starts
  (bind _outactors (Actor|GetAllActorswithTag "Platform"))
  (Variables|Default|SettotalPlatforms (Utilities|Array|Length _outactors)))

(event EventDestroyed
  ;[1 1 1] When a platform is destroyed, add on to "Destroyed Platforms" list
  (Variables|Default|SetDestroyedPlatforms (+ (Variables|Default|GetDestroyedPlatforms) 1))
  (Development|PrintString (Utilities|String|ToString(Integer) (Variables|Default|GetDestroyedPlatforms)))
  ;[1 1 1] If "Destroyed Platforms" and "Total Platforms" are equal, WIN
  (if (== (Variables|Default|GetDestroyedPlatforms) (Variables|Default|GettotalPlatforms))
    _))

(fn ConstructionScript)