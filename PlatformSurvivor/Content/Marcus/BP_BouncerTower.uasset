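; BP_BouncerTower is a bouncer that knocks away any Character that begins overlapping its Capsule.
; It launches the Character along the normalized direction from the tower's root to the overlapping component, scaled by PushForceVar and overriding existing velocity on all axes.
; Each bounce spawns the P_Bounce particle effect attached to the Capsule.
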(event OnComponentBeginOverlap(Capsule)
  (params (OverlappedComponent :type Primitive%20Component%20Object%20Reference) (OtherActor :type Actor%20Object%20Reference) (OtherComp :type Primitive%20Component%20Object%20Reference) (OtherBodyIndex :type Integer) (bFromSweep :type Boolean) (SweepResult :type Hit%20Result%20Structure%20%28by%20ref%29))
  (bind _returnvalue (Transformation|GetWorldLocation OtherComp))
  (bind _defaultsceneroot (Variables|Default|GetDefaultSceneRoot))
  (bind _pushforcevar (Variables|Default|GetPushForceVar))
  (bind _returnvalue_2 (Transformation|GetWorldLocation _defaultsceneroot))
  (bind _returnvalue_3 (- _returnvalue _returnvalue_2))
  (bind _returnvalue_4 (Math|Vector|Normalize _returnvalue_3))
  (bind _returnvalue_5 (* _returnvalue_4 _pushforcevar))
  ;[1 1 1] Affect Character
  (bind _ascharacter (Utilities|Casting|CastToCharacter OtherActor))
  (Character|LaunchCharacter _ascharacter (Math|Vector|MakeVector (.x _returnvalue_5) (.y _returnvalue_5) (.z _returnvalue_5)) true true)
  (Effects|SpawnEmitterAttached "/Game/Marcus/P_Bounce.P_Bounce" (Variables|Default|GetCapsule) "None"))

(fn ConstructionScript)