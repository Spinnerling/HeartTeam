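; BP_LoseBox is a lose trigger that ends the attempt and restarts the level when the player overlaps its CollisionBox.
; On overlap it moves the first TopDownCharacter to a hard-coded location out of the way.
; A timeline then lerps the LoseText on MainCamera_BP from TextOriginSpace to TextSpace, and reopens the current level by name when it finishes.
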(event OnComponentBeginOverlap(CollisionBox)
  (params (OverlappedComponent :type Primitive%20Component%20Object%20Reference) (OtherActor :type Actor%20Object%20Reference) (OtherComp :type Primitive%20Component%20Object%20Reference) (OtherBodyIndex :type Integer) (bFromSweep :type Boolean) (SweepResult :type Hit%20Result%20Structure%20%28by%20ref%29))
  ;[1 1 1] Check for Player
  (if (== OtherActor (Game|GetPlayerCharacter 0))
    ;[1 1 1] Teleport character away
    (bind _outactors (Actor|GetAllActorsOfClass "/Game/TopDownBP/Blueprints/TopDownCharacter.TopDownCharacter_C"))
    (Transformation|SetWorldLocation (Variables|/Script/Engine.Actor|GetRootComponent (Utilities|Array|Get(acopy) _outactors)) "-1920.000000,-260.000000,1100.000000" false false)
    ;[1 1 1] Show Lose Text
    (bind _outactors_2 (Actor|GetAllActorsOfClass "/Game/Benjamin/MainCamera_BP.MainCamera_BP_C"))
    (bind _newtrack_2 (Timeline|Timeline_0 PlayFromStart)
      (:Update
        (Transformation|SetWorldLocation (Variables|/Game/Benjamin/MainCamera_BP.MainCamera_BP_C|GetLoseText (Utilities|Array|Get(acopy) _outactors_2)) (Math|Vector|Lerp(Vector) (Transformation|GetWorldLocation (Variables|/Game/Benjamin/MainCamera_BP.MainCamera_BP_C|GetTextOriginSpace (Utilities|Array|Get(acopy) _outactors_2))) (Transformation|GetWorldLocation (Variables|/Game/Benjamin/MainCamera_BP.MainCamera_BP_C|GetTextSpace (Utilities|Array|Get(acopy) _outactors_2))) _newtrack_2) false false))
      (:Finished
        ;[1 1 1] Reset Level
        (bind _returnvalue (Game|GetCurrentLevelName true))
        (Game|OpenLevel(byName) (Utilities|String|StringToName _returnvalue))))))

(fn ConstructionScript)