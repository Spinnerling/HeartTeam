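; BP_TurningPlatform is a platform that flips over when an actor implementing BPI_Player overlaps its Box trigger.
; The TurnOver timeline drives the root component's world pitch, with roll and yaw held at zero.
; In parallel, delays briefly disable the Platform's collision during the rotation, then restore it.
; A DoOnce blocks retriggering until the timeline finishes and resets it.
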(event OnComponentBeginOverlap(Box)
  (params (OverlappedComponent :type Primitive%20Component%20Object%20Reference) (OtherActor :type Actor%20Object%20Reference) (OtherComp :type Primitive%20Component%20Object%20Reference) (OtherBodyIndex :type Integer) (bFromSweep :type Boolean) (SweepResult :type Hit%20Result%20Structure%20%28by%20ref%29))
  (if (Utilities|DoesObjectImplementInterface OtherActor "/Game/OurStuff/Blueprints/BPI_Player.BPI_Player_C")
    (Utilities|FlowControl|DoOnce false :!label _label
      (:Completed
        (Utilities|FlowControl|Sequence
          (:then_0
            ;[1 1 1] Turn off collision during rotation
            (Utilities|FlowControl|Delay 0.5)
            (Collision|SetCollisionEnabled (Variables|Default|GetPlatform) "NoCollision")
            (Utilities|FlowControl|Delay 1.0)
            (Collision|SetCollisionEnabled (Variables|Default|GetPlatform) "QueryAndPhysics"))
          (:then_1
            ;[1 1 1] Rotate platform
            (bind _timertrack (Timeline|Turn%20Over PlayFromStart)
              (:Update
                (Transformation|SetWorldRotation (Variables|Default|GetDefaultSceneRoot) (Math|Rotator|MakeRotator 0.0 _timertrack 0.0) false false))
              (:Finished
                (goto _label Reset)))))))))

(fn ConstructionScript)