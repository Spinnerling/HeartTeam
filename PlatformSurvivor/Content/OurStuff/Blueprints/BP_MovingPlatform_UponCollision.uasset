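; Moving platform that travels along a spline while the player stands in its trigger box.
; On begin play, the platform takes the spline's starting yaw and roll, with pitch held flat.
; When the player character enters the box, a timeline drives the platform's location and rotation along the spline length.
; When the player leaves the box, the timeline reverses, sending the platform back toward the start.
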(event OnComponentBeginOverlap(Box)
  (params (OverlappedComponent :type Primitive%20Component%20Object%20Reference) (OtherActor :type Actor%20Object%20Reference) (OtherComp :type Primitive%20Component%20Object%20Reference) (OtherBodyIndex :type Integer) (bFromSweep :type Boolean) (SweepResult :type Hit%20Result%20Structure%20%28by%20ref%29))
  (bind _spline (Variables|Default|GetSpline))
  (if (== OtherActor (Game|GetPlayerCharacter 0))
    (bind _newtrack_0 (Timeline|MovePlatformOnCollision Play)
      (:Update
        ;[1 1 1] Platform follows Spline to Destination
        (Transformation|SetWorldLocation (Variables|Default|GetPlatform) (Spline|GetLocationatDistanceAlongSpline _spline (* _newtrack_0 (Spline|GetSplineLength (Variables|Default|GetSpline))) "World") false false)
        (Transformation|SetRelativeRotation (Variables|Default|GetPlatform) (Math|Rotator|MakeRotator (.roll (Spline|GetRotationatDistanceAlongSpline _spline (* _newtrack_0 (Spline|GetSplineLength (Variables|Default|GetSpline))) "Local")) 0.0 (.yaw (Spline|GetRotationatDistanceAlongSpline _spline (* _newtrack_0 (Spline|GetSplineLength (Variables|Default|GetSpline))) "Local"))) false false)))))

(event OnComponentEndOverlap(Box)
  (params (OverlappedComponent :type Primitive%20Component%20Object%20Reference) (OtherActor :type Actor%20Object%20Reference) (OtherComp :type Primitive%20Component%20Object%20Reference) (OtherBodyIndex :type Integer))
  (bind _spline (Variables|Default|GetSpline))
  (if (== (Game|GetPlayerCharacter 0) OtherActor)
    (bind _newtrack_0 (Timeline|MovePlatformOnCollision Reverse)
      (:Update
        ;[1 1 1] Platform follows Spline to Destination
        (Transformation|SetWorldLocation (Variables|Default|GetPlatform) (Spline|GetLocationatDistanceAlongSpline _spline (* _newtrack_0 (Spline|GetSplineLength (Variables|Default|GetSpline))) "World") false false)
        (Transformation|SetRelativeRotation (Variables|Default|GetPlatform) (Math|Rotator|MakeRotator (.roll (Spline|GetRotationatDistanceAlongSpline _spline (* _newtrack_0 (Spline|GetSplineLength (Variables|Default|GetSpline))) "Local")) 0.0 (.yaw (Spline|GetRotationatDistanceAlongSpline _spline (* _newtrack_0 (Spline|GetSplineLength (Variables|Default|GetSpline))) "Local"))) false false)))))

(event EventBeginPlay
  (bind _spline (Variables|Default|GetSpline))
  (bind _returnvalue (Spline|GetRotationatDistanceAlongSpline _spline 0.0 "Local"))
  ;[1 1 1] Rotates Platform Along Spline
  (Transformation|SetRelativeRotation (Variables|Default|GetPlatform) (Math|Rotator|MakeRotator (.roll _returnvalue) 0.0 (.yaw _returnvalue)) false false))

(fn ConstructionScript)