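; Home platform that acts as the level's win point, requiring the player on it and all platforms destroyed.
; Box overlaps and an AllPlatformsDestroyed event set two flags, so either condition can complete last and trigger the win.
; A timeline slides the MainCamera_BP win text into view between two anchors, then opens NextLevelName.
; The on-platform flag follows any actor's overlap, as it is set before the player check.
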(event OnComponentBeginOverlap(Box)
  (params (OverlappedComponent :type Primitive%20Component%20Object%20Reference) (OtherActor :type Actor%20Object%20Reference) (OtherComp :type Primitive%20Component%20Object%20Reference) (OtherBodyIndex :type Integer) (bFromSweep :type Boolean) (SweepResult :type Hit%20Result%20Structure%20%28by%20ref%29))
  ;[1 1 1] Win condition
  (Variables|Default|SetplayerOnPlatform true)
  ;;[1 1 1] Check for player
  (if (== OtherActor (Game|GetPlayerCharacter 0))
    (if (Variables|Default|Getplatformsdestroyed)
      ;;[1 1 1] Show Win Text
      (bind _outactors (Actor|GetAllActorsOfClass "/Game/Benjamin/MainCamera_BP.MainCamera_BP_C"))
      (bind _newtrack_2 (Timeline|Timeline_0 PlayFromStart)
        (:Update
          (Transformation|SetWorldLocation (Variables|/Game/Benjamin/MainCamera_BP.MainCamera_BP_C|GetWinText (Utilities|Array|Get(acopy) _outactors)) (Math|Vector|Lerp(Vector) (Transformation|GetWorldLocation (Variables|/Game/Benjamin/MainCamera_BP.MainCamera_BP_C|GetTextOriginSpace (Utilities|Array|Get(acopy) _outactors))) (Transformation|GetWorldLocation (Variables|/Game/Benjamin/MainCamera_BP.MainCamera_BP_C|GetTextSpace (Utilities|Array|Get(acopy) _outactors))) _newtrack_2) false false))
        (:Finished
          (Game|OpenLevel(byName) (Variables|Default|GetNextLevelName)))))))

(event OnComponentEndOverlap(Box)
  (params (OverlappedComponent :type Primitive%20Component%20Object%20Reference) (OtherActor :type Actor%20Object%20Reference) (OtherComp :type Primitive%20Component%20Object%20Reference) (OtherBodyIndex :type Integer))
  (Variables|Default|SetplayerOnPlatform false))

(event Custom|All%20Platforms%20Destroyed
  ;[1 1 1] Win condition
  (Variables|Default|Setplatformsdestroyed true)
  (if (Variables|Default|GetplayerOnPlatform)
    ;;[1 1 1] Show Win Text
    (bind _outactors (Actor|GetAllActorsOfClass "/Game/Benjamin/MainCamera_BP.MainCamera_BP_C"))
    (bind _newtrack_2 (Timeline|Timeline_0 PlayFromStart)
      (:Update
        (Transformation|SetWorldLocation (Variables|/Game/Benjamin/MainCamera_BP.MainCamera_BP_C|GetWinText (Utilities|Array|Get(acopy) _outactors)) (Math|Vector|Lerp(Vector) (Transformation|GetWorldLocation (Variables|/Game/Benjamin/MainCamera_BP.MainCamera_BP_C|GetTextOriginSpace (Utilities|Array|Get(acopy) _outactors))) (Transformation|GetWorldLocation (Variables|/Game/Benjamin/MainCamera_BP.MainCamera_BP_C|GetTextSpace (Utilities|Array|Get(acopy) _outactors))) _newtrack_2) false false))
      (:Finished
        (Game|OpenLevel(byName) (Variables|Default|GetNextLevelName))))))

(fn ConstructionScript)