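; BP_DoorSwitch is a color-coded trigger switch that signals a target actor when the player steps into it.
; On BeginPlay it creates a dynamic material on its Cone and sets the emissive color to one of four presets chosen by ColorTracker.
; When the player character overlaps the Box, it calls SwitchOnOffMessage on Target with true; it never sends an off signal.
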(event OnComponentBeginOverlap(Box)
  (params (OverlappedComponent :type Primitive%20Component%20Object%20Reference) (OtherActor :type Actor%20Object%20Reference) (OtherComp :type Primitive%20Component%20Object%20Reference) (OtherBodyIndex :type Integer) (bFromSweep :type Boolean) (SweepResult :type Hit%20Result%20Structure%20%28by%20ref%29))
  (if (== OtherActor (Game|GetPlayerCharacter 0))
    (Class|BPIDoorOpenSwitch|SwitchOn/Off(Message) (Variables|Default|GetTarget) true)))

(event EventBeginPlay
  (bind _returnvalue (Rendering|Material|CreateDynamicMaterialInstance (Variables|Default|GetCone) 0 0 "None" :!class /Script/Engine.PrimitiveComponent))
  (bind _output_get (Variables|Default|SetMaterialRefrence _returnvalue))
  (switch int (Variables|Default|GetColorTracker)
    (:0
      (Rendering|Material|SetVectorParameterValue _output_get "EmissiveColor" "(R=0.057249,G=1.000000,B=0.000000,A=1.000000)" :!class /Script/Engine.MaterialInstanceDynamic))
    (:1
      (Rendering|Material|SetVectorParameterValue _output_get "EmissiveColor" "(R=1.000000,G=0.000000,B=0.901285,A=1.000000)" :!class /Script/Engine.MaterialInstanceDynamic))
    (:2
      (Rendering|Material|SetVectorParameterValue _output_get "EmissiveColor" "(R=0.000000,G=0.967913,B=1.000000,A=1.000000)" :!class /Script/Engine.MaterialInstanceDynamic))
    (:3
      (Rendering|Material|SetVectorParameterValue _output_get "EmissiveColor" "(R=1.000000,G=0.398821,B=0.000000,A=1.000000)" :!class /Script/Engine.MaterialInstanceDynamic))))

(fn ConstructionScript)