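; Moving platform that starts travelling along its spline as soon as play begins, with no trigger needed.
; The MovePlatformOnCollision timeline's track scales the spline length into a distance that sets the platform's world location without sweep.
; Relative rotation follows the spline's local roll and yaw, with pitch held at zero.
; When the timeline finishes, Revers only calls Reverse, never Play again.
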(event Custom|Revers
  (bind _spline (Variables|Default|GetSpline))
  (bind _newtrack_0 (Timeline|MovePlatformOnCollision Reverse)
    (:Update
      ;[1 1 1] Platform follows Spline to Destination
      (Transformation|SetWorldLocation (Variables|Default|GetPlatform) (Spline|GetLocationatDistanceAlongSpline _spline (* _newtrack_0 (Spline|GetSplineLength (Variables|Default|GetSpline))) "World") false false)
      (Transformation|SetRelativeRotation (Variables|Default|GetPlatform) (Math|Rotator|MakeRotator (.roll (Spline|GetRotationatDistanceAlongSpline _spline (* _newtrack_0 (Spline|GetSplineLength (Variables|Default|GetSpline))) "Local")) 0.0 (.yaw (Spline|GetRotationatDistanceAlongSpline _spline (* _newtrack_0 (Spline|GetSplineLength (Variables|Default|GetSpline))) "Local"))) false false))
    (:Finished
      (CallFunction|Revers))))

(event EventBeginPlay
  (bind _spline (Variables|Default|GetSpline))
  (bind _spline_2 (Variables|Default|GetSpline))
  (bind _returnvalue (Spline|GetRotationatDistanceAlongSpline _spline_2 0.0 "Local"))
  ;[1 1 1] Rotates Platform Along Spline
  (Transformation|SetRelativeRotation (Variables|Default|GetPlatform) (Math|Rotator|MakeRotator (.roll _returnvalue) 0.0 (.yaw _returnvalue)) false false)
  (bind _newtrack_0 (Timeline|MovePlatformOnCollision Play)
    (:Update
      ;[1 1 1] Platform follows Spline to Destination
      (Transformation|SetWorldLocation (Variables|Default|GetPlatform) (Spline|GetLocationatDistanceAlongSpline _spline (* _newtrack_0 (Spline|GetSplineLength (Variables|Default|GetSpline))) "World") false false)
      (Transformation|SetRelativeRotation (Variables|Default|GetPlatform) (Math|Rotator|MakeRotator (.roll (Spline|GetRotationatDistanceAlongSpline _spline (* _newtrack_0 (Spline|GetSplineLength (Variables|Default|GetSpline))) "Local")) 0.0 (.yaw (Spline|GetRotationatDistanceAlongSpline _spline (* _newtrack_0 (Spline|GetSplineLength (Variables|Default|GetSpline))) "Local"))) false false))
    (:Finished
      (CallFunction|Revers))))

(fn ConstructionScript)