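; BP_Door is a colour-coded door that slides along a spline when switched on.
; BeginPlay creates a dynamic material on the Door component and sets one of four emissive colours from ColourTracker.
; SwitchOn/Off plays the DoorONOff timeline when passed true, mapping its value to spline distance to drive the door's position and pitch.
; The false input has no logic, so the event never closes the door.
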(event EventBeginPlay
  (bind _returnvalue (Rendering|Material|CreateDynamicMaterialInstance (Variables|Default|GetDoor) 0 0 "None" :!class /Script/Engine.PrimitiveComponent))
  (bind _output_get (Variables|Default|SetMaterialReference _returnvalue))
  (switch int (Variables|Default|GetColourTracker)
    (:0
      (Rendering|Material|SetVectorParameterValue _output_get "EmissiveColor" "(R=0.057249,G=1.000000,B=0.000000,A=1.000000)" :!class /Script/Engine.MaterialInstanceDynamic))
    (:1
      (Rendering|Material|SetVectorParameterValue _output_get "EmissiveColor" "(R=1.000000,G=0.000000,B=0.901285,A=1.000000)" :!class /Script/Engine.MaterialInstanceDynamic))
    (:2
      (Rendering|Material|SetVectorParameterValue _output_get "EmissiveColor" "(R=0.000000,G=0.967913,B=1.000000,A=1.000000)" :!class /Script/Engine.MaterialInstanceDynamic))
    (:3
      (Rendering|Material|SetVectorParameterValue _output_get "EmissiveColor" "(R=1.000000,G=0.398821,B=0.000000,A=1.000000)" :!class /Script/Engine.MaterialInstanceDynamic))))

(event EventSwitchOn/Off
  (params (ON/OFF :type Boolean))
  (bind _spline (Variables|Default|GetSpline))
  (if ON/OFF
    (Transformation|SetRelativeRotation (Variables|Default|GetDoor) (Math|Rotator|MakeRotator 0.0 (.pitch (Spline|GetRotationatDistanceAlongSpline (Variables|Default|GetSpline) 0.0 "Local")) 0.0) false false)
    (bind _dooropen_close (Timeline|DoorON/Off Play)
      (:Update
        (Transformation|SetWorldLocation (Variables|Default|GetDoor) (Spline|GetLocationatDistanceAlongSpline _spline (* _dooropen_close (Spline|GetSplineLength (Variables|Default|GetSpline))) "World") false false)
        (Transformation|SetRelativeRotation (Variables|Default|GetDoor) (Math|Rotator|MakeRotator 0.0 (.pitch (Spline|GetRotationatDistanceAlongSpline _spline (* _dooropen_close (Spline|GetSplineLength (Variables|Default|GetSpline))) "Local")) 0.0) false false)))))

(fn ConstructionScript)