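; BP_DestroyablePlatform is a platform actor that destroys itself after the player touches its trigger box.
; On overlap with an actor implementing BPI_Player, it switches on the platform material's emissive and plays a timeline that drives the TimeMult parameter.
; When the timeline finishes, it notifies the first actor tagged PlatformMaster through DestroyedMessage, then destroys itself.
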(event OnComponentBeginOverlap(Box)
  (params (OverlappedComponent :type Primitive%20Component%20Object%20Reference) (OtherActor :type Actor%20Object%20Reference) (OtherComp :type Primitive%20Component%20Object%20Reference) (OtherBodyIndex :type Integer) (bFromSweep :type Boolean) (SweepResult :type Hit%20Result%20Structure%20%28by%20ref%29))
  (if (Utilities|DoesObjectImplementInterface OtherActor "/Game/OurStuff/Blueprints/BPI_Player.BPI_Player_C")
    (Rendering|Material|SetScalarParameterValueonMaterials (Variables|Default|GetPlatform) "Emissive ONOFF" 1.0)
    (bind _timertrack (Timeline|Timer Play)
      (:Update
        (Rendering|Material|SetScalarParameterValueonMaterials (Variables|Default|GetPlatform) "TimeMult" _timertrack))
      (:Finished
        (bind _outactors (Actor|GetAllActorswithTag "PlatformMaster"))
        (Class|BPIPlatforms|Destroyed(Message) (Utilities|Array|Get(acopy) _outactors))
        (Actor|DestroyActor)))))

(fn ConstructionScript)