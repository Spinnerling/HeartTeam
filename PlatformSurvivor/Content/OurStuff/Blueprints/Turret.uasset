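; Turret Blueprint that tracks the player character and fires at it when within range.
; Each tick it updates an in-range flag from distance and smoothly rotates the barrels toward the player using interpolated look-at pitch and yaw.
; A self-calling event started at BeginPlay spawns bullets from the Barrel_1 socket at the fire rate, or rechecks periodically while the player is out of range.
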(event Custom|TurretRotation
  (bind _returnvalue (Game|GetPlayerCharacter 0))
  (bind _barrels (Variables|Default|GetBarrels))
  (bind _returnvalue_2 (Transformation|GetWorldLocation _barrels))
  (bind _returnvalue_3 (Transformation|GetActorLocation _returnvalue))
  (bind _returnvalue_4 (Math|Rotator|FindLookatRotation _returnvalue_2 _returnvalue_3))
  (bind (_roll _pitch _yaw) (Math|Rotator|BreakRotator _returnvalue_4))
  ;[1 0 0] TurretFollowsPlayer
  (if (Variables|Default|GetInRange)
    (Transformation|SetWorldRotation (Variables|Default|GetBarrels) (Math|Interpolation|RInterpTo (Transformation|GetWorldRotation (Variables|Default|GetBarrels)) (Math|Rotator|MakeRotator 0.0 _pitch _yaw) (Variables|Default|GetDeltaTime) (Variables|Default|GetRotationSpeed)) false false)))

(event Custom|TurretRange
  ;[1 0.894 0.03957] TurretRange
  (if (< (Transformation|GetDistanceTo self (Game|GetPlayerCharacter 0)) (Variables|Default|GetAttackRange))
    (Variables|Default|SetInRange true)
    (else
      (Variables|Default|SetInRange false))))

(event Custom|TurretShootAtPlayer
  ;[0.1085 0.04025 1] Turret Shoots Player
  (if (Variables|Default|GetInRange)
    (Game|SpawnActorfromClass "/Game/Jack/Turret_Bullets.Turret_Bullets_C" (Transformation|GetSocketTransform (Variables|Default|GetBarrels) "Barrel_1" "RTS_World") "Undefined" 0 0)
    (Utilities|FlowControl|RetriggerableDelay (Variables|Default|GetFireRate))
    (CallFunction|TurretShootatPlayer)
    (else
      (Utilities|FlowControl|RetriggerableDelay 0.5)
      (CallFunction|TurretShootatPlayer))))

(event EventBeginPlay
  (CallFunction|TurretShootatPlayer))

(event EventTick
  (params (DeltaSeconds :type Float%20%28single-precision%29))
  ;[1 0 0] TurretFollowsPlayer
  (Variables|Default|SetDeltaTime DeltaSeconds)
  (CallFunction|TurretRotation)
  (CallFunction|TurretRange))

(fn ConstructionScript)