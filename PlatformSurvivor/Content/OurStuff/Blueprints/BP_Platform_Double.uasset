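; Platform that survives one player step and destroys itself after a second.
; It starts green through a dynamic material instance and turns yellow when an actor implementing BPI_Player overlaps it.
; On a later overlap it enables emissive and plays a timeline that drives the material's TimeMult parameter.
; When the timeline finishes, it sends DestroyedMessage to the first actor tagged PlatformMaster, then destroys itself.
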(event OnComponentBeginOverlap(Col)
  (params (OverlappedComponent :type Primitive%20Component%20Object%20Reference) (OtherActor :type Actor%20Object%20Reference) (OtherComp :type Primitive%20Component%20Object%20Reference) (OtherBodyIndex :type Integer) (bFromSweep :type Boolean) (SweepResult :type Hit%20Result%20Structure%20%28by%20ref%29))
  (if (Utilities|DoesObjectImplementInterface OtherActor "/Game/OurStuff/Blueprints/BPI_Player.BPI_Player_C")
    (Rendering|Material|SetVectorParameterValue (Variables|Default|GetPlatformMaterialRef) "BaseColor" "(R=1.000000,G=0.935929,B=0.092793,A=1.000000)" :!class /Script/Engine.MaterialInstanceDynamic)
    (if (Variables|Default|GetHasSteppedOn)
      (Rendering|Material|SetScalarParameterValueonMaterials (Variables|Default|GetCube) "Emissive ONOFF" 1.0)
      (bind _timertrack (Timeline|Timeline_0 Play)
        (:Update
          (Rendering|Material|SetScalarParameterValueonMaterials (Variables|Default|GetCube) "TimeMult" _timertrack))
        (:Finished
          (bind _outactors (Actor|GetAllActorswithTag "PlatformMaster"))
          (Class|BPIPlatforms|Destroyed(Message) (Utilities|Array|Get(acopy) _outactors))
          (Actor|DestroyActor)))
      (else
        (Variables|Default|SetHasSteppedOn true)))))

(event EventBeginPlay
  (bind _returnvalue (Rendering|Material|CreateDynamicMaterialInstance (Variables|Default|GetCube) 0 "/Game/OurStuff/Materials/All/Mat_Double_Platform.Mat_Double_Platform" "None" :!class /Script/Engine.PrimitiveComponent))
  (Variables|Default|SetPlatformMaterialRef _returnvalue)
  (Rendering|Material|SetVectorParameterValue (Variables|Default|GetPlatformMaterialRef) "BaseColor" "(R=0.085571,G=1.000000,B=0.063079,A=1.000000)" :!class /Script/Engine.MaterialInstanceDynamic))

(fn ConstructionScript)